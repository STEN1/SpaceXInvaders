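; BP_SpaceXGameModeBase is a game mode Blueprint that manages the HUD and game-over screen.
; On game start it creates the ship-count and health bar widgets, seeding the count from GetNumberOfShips.
; Update events find those widgets by class to refresh the ship count and health bar.
; On game over it shows a WBP_GameOver widget with text set by whether the player won.
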(event EventUpdateShips
  (bind _foundwidgets (Widget|GetAllWidgetsOfClass "/Game/Widgets/WBP_Ships.WBP_Ships_C" true))
  (Default|SetShips _foundwidgets (Class|SpaceXGameModeBase|GetNumberOfShips)))

(event EventUpdateHealthUI
  (params (Health :type Float%20%28single-precision%29) (DefaultHealth :type Float%20%28single-precision%29))
  (bind _foundwidgets (Widget|GetAllWidgetsOfClass "/Game/Widgets/WBP_Health.WBP_Health_C" true))
  (Default|SetHealthBar _foundwidgets Health DefaultHealth))

(event EventGameStart
  (bind _returnvalue (UserInterface|CreateWidget "/Game/Widgets/WBP_Ships.WBP_Ships_C"))
  (Default|SetShips _returnvalue (Class|SpaceXGameModeBase|GetNumberOfShips))
  (UserInterface|Viewport|AddtoViewport _returnvalue 0)
  (bind _returnvalue_2 (UserInterface|CreateWidget "/Game/Widgets/WBP_Health.WBP_Health_C"))
  (UserInterface|Viewport|AddtoViewport _returnvalue_2 0))

(event EventGameOver
  (params (PlayerWon :type Boolean))
  (bind _returnvalue (UserInterface|CreateWidget "/Game/Widgets/WBP_GameOver.WBP_GameOver_C"))
  (Default|SetGameOverText _returnvalue PlayerWon)
  (UserInterface|Viewport|AddtoViewport _returnvalue 0))

(fn ConstructionScript)